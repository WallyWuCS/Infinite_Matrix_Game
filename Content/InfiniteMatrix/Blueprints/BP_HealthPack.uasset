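; BP_HealthPack is a short-lived health pickup that destroys itself after a fixed delay from BeginPlay.
; When BP_Player overlaps its Collision component with health below maximum, it calls the player's IncrementHealth, without destroying the pack.
; RandomizeHealthpack, not called within this Blueprint, applies a fixed health-colored material to Collision despite its name.
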(event OnComponentBeginOverlap(Collision)
  (params (OverlappedComponent :type Primitive%20Component%20Object%20Reference) (OtherActor :type Actor%20Object%20Reference) (OtherComp :type Primitive%20Component%20Object%20Reference) (OtherBodyIndex :type Integer) (bFromSweep :type Boolean) (SweepResult :type Hit%20Result%20Structure%20%28by%20ref%29))
  (bind _asbp_player (Utilities|Casting|CastToBP_Player OtherActor))
  (Math|Integer|CompareInt (Variables|/Game/InfiniteMatrix/Blueprints/BP_Player.BP_Player_C|GetCurrentHealth _asbp_player) (Variables|/Game/InfiniteMatrix/Blueprints/BP_Player.BP_Player_C|GetMaxHealth _asbp_player)
    (:<
      (Default|IncrementHealth _asbp_player))))

(event EventBeginPlay
  (Utilities|FlowControl|Delay 1e+01)
  (Actor|DestroyActor))

(event EventTick
  (params (DeltaSeconds :type Float%20%28single-precision%29)))

(fn ConstructionScript)

(fn RandomizeHealthpack
  (Rendering|Material|SetMaterial (Variables|Default|GetCollision) 0 "/Game/InfiniteMatrix/Materials/MI_Color_Health.MI_Color_Health"))